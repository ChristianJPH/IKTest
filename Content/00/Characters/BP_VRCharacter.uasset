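; VR player character with head-relative smooth locomotion, smooth turning and jumping.
; Each tick recenters the capsule under the HMD, counter-offsetting VROrigin, and scales its height to the camera, capped by a player height sampled after a startup delay.
; The local player sends quantized head and controller transforms, plus a byte-sized capsule height, to the server on a timer.
; Non-local instances interpolate capsule, camera and controllers toward those stored values.
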(event Custom|Tracker%20Replication
  ;[0.15 0.15 0.15 0.5] Data replication to server
  (if (Pawn|IsLocallyControlled)
    (Utilities|Time|SetTimerbyEvent (delegate Custom|Replicate%20Transforms) (/ 1.0 (Variables|Default|GetTracker%20Replication%20Frecuency)) true)))

(event Custom|Replicate%20Transforms
  (bind _camera (Variables|Default|GetCamera))
  (bind _leftmotioncontroller (Variables|Default|GetLeftMotionController))
  (bind _rightmotioncontroller (Variables|Default|GetRightMotionController))
  (bind _returnvalue (Transformation|GetWorldTransform _camera))
  (bind _returnvalue_2 (Transformation|GetWorldTransform _leftmotioncontroller))
  (bind _returnvalue_3 (Transformation|GetWorldTransform _rightmotioncontroller))
  ;[0.15 0.15 0.15 0.5] Data replication to server
  (CallFunction|VRTransformstoServer (Utilities|Array|MakeArray (Math|Vector|MakeVectorNetQuantize (.x (.location _returnvalue)) (.y (.location _returnvalue)) (.z (.location _returnvalue))) (Math|Vector|MakeVectorNetQuantize (.x (.location _returnvalue_2)) (.y (.location _returnvalue_2)) (.z (.location _returnvalue_2))) (Math|Vector|MakeVectorNetQuantize (.x (.location _returnvalue_3)) (.y (.location _returnvalue_3)) (.z (.location _returnvalue_3)))) (Utilities|Array|MakeArray (.rotation _returnvalue) (.rotation _returnvalue_2) (.rotation _returnvalue_3)) (Math|Conversions|ToByte(Integer) (Math|Float|Round (Math|Float|Clamp(Float) (- (.z (.location _returnvalue)) (.z (.location (Transformation|GetWorldTransform (Variables|Collision|GetCapsuleComponent))))) 0.0 255.0)))))

(event Custom|Interpolate%20Tracking%20Sources
  (bind _returnvalue (Utilities|Time|GetWorldDeltaSeconds))
  (bind _leftmotioncontroller (Variables|Default|GetLeftMotionController))
  (bind _rightmotioncontroller (Variables|Default|GetRightMotionController))
  (bind _tracker_replication_frecuency (Variables|Default|GetTracker%20Replication%20Frecuency))
  (bind _capsulecomponent (Variables|Collision|GetCapsuleComponent))
  (bind _camera (Variables|Default|GetCamera))
  (bind _vr_locations (Variables|Default|GetVR%20Locations))
  (bind _vr_rotations (Variables|Default|GetVR%20Rotations))
  (bind _returnvalue_2 (Transformation|GetWorldTransform _camera))
  (bind _returnvalue_3 (Transformation|GetWorldTransform _capsulecomponent))
  (bind _output (Utilities|Array|Get(acopy) _vr_locations))
  (bind _output_2 (Utilities|Array|Get(acopy) _vr_rotations))
  (bind _returnvalue_4 (Class|KismetMathLibrary|TInterpto _returnvalue_2 (Math|Transform|MakeTransform _output _output_2 "1.000000,1.000000,1.000000") _returnvalue _tracker_replication_frecuency))
  (bind _location (Math|Transform|BreakTransform _returnvalue_4))
  (if (not (Pawn|IsLocallyControlled))
    (Transformation|SetWorldTransform _capsulecomponent (Class|KismetMathLibrary|TInterpto (Math|Transform|MakeTransform (Math|Vector|MakeVector (.x _location) (.y _location) (.z (.location _returnvalue_3))) (.rotation _returnvalue_3) "1.000000,1.000000,1.000000") (Math|Transform|MakeTransform (Math|Vector|MakeVector (.x _location) (.y _location) (- (.z _location) (Variables|Default|GetCapsule%20Z%20Relative))) (.rotation _returnvalue_3) "1.000000,1.000000,1.000000") (Utilities|Time|GetWorldDeltaSeconds) (Variables|Default|GetTracker%20Replication%20Frecuency)) false false)
    (Components|Capsule|SetCapsuleHalfHeight (Variables|Collision|GetCapsuleComponent) (Math|Conversions|ToFloat(Byte) (Variables|Default|GetCapsule%20Z%20Relative)) false)
    (Transformation|SetWorldTransform _camera _returnvalue_4 false false)
    (Transformation|SetWorldTransform _leftmotioncontroller (Class|KismetMathLibrary|TInterpto (Transformation|GetWorldTransform _leftmotioncontroller) (Math|Transform|MakeTransform (Utilities|Array|Get(acopy) _vr_locations 1) (Utilities|Array|Get(acopy) _vr_rotations 1) "1.000000,1.000000,1.000000") (Utilities|Time|GetWorldDeltaSeconds) (Variables|Default|GetTracker%20Replication%20Frecuency)) false false)
    (Transformation|SetWorldTransform _rightmotioncontroller (Class|KismetMathLibrary|TInterpto (Transformation|GetWorldTransform _rightmotioncontroller) (Math|Transform|MakeTransform (Utilities|Array|Get(acopy) _vr_locations 2) (Utilities|Array|Get(acopy) _vr_rotations 2) "1.000000,1.000000,1.000000") (Utilities|Time|GetWorldDeltaSeconds) (Variables|Default|GetTracker%20Replication%20Frecuency)) false false)))

(event Custom|VR%20Transforms%20to%20Server
  (params (Locations :type Array%20of%20Vector%20Net%20Quantize%20Structures) (Rotations :type Array%20of%20Rotators) (Capsule%20Z%20Relative :type Byte))
  ;[0.15 0.15 0.15 0.5] Replicating transform of Character
  (Variables|Default|SetVR%20Locations Locations)
  (Variables|Default|SetVR%20Rotations Rotations)
  (Variables|Default|SetCapsule%20Z%20Relative Capsule%20Z%20Relative))

(event Input|EnhancedActionEvents|EnhancedInputActionIA_SmoothTurn
  (params (ActionValue :type Float%20%28double-precision%29) (ElapsedSeconds :type Float%20%28double-precision%29) (TriggeredSeconds :type Float%20%28double-precision%29) (InputAction :type Input%20Action%20Object%20Reference :default "/Game/00/Inputs/IA_SmoothTurn.IA_SmoothTurn"))
  (Pawn|Input|AddControllerYawInput (* ActionValue (Variables|Default|GetSmooth%20Turn%20Speed))))

(event Input|EnhancedActionEvents|EnhancedInputActionIA_SmoothMovement
  (params (ActionValue :type Vector%202D%20Structure) (ElapsedSeconds :type Float%20%28double-precision%29) (TriggeredSeconds :type Float%20%28double-precision%29) (InputAction :type Input%20Action%20Object%20Reference :default "/Game/00/Inputs/IA_SmoothMovement.IA_SmoothMovement"))
  (bind _camera (Variables|Default|GetCamera))
  (bind _returnvalue (Math|Vector|GetForwardVector _camera))
  (bind _returnvalue_2 (Math|Vector|GetRightVector _camera))
  (bind _returnvalue_3 (Math|Vector|Normalize _returnvalue_2))
  (bind _returnvalue_4 (Math|Vector|Normalize _returnvalue))
  (Pawn|Input|AddMovementInput (Math|Vector|MakeVector (.x _returnvalue_4) (.y _returnvalue_4) 0.0) (.y ActionValue) false)
  (Pawn|Input|AddMovementInput (Math|Vector|MakeVector (.x _returnvalue_3) (.y _returnvalue_3) 0.0) (.x ActionValue) false))

(event Input|EnhancedActionEvents|EnhancedInputActionIA_Jump
  (params (ActionValue :type Boolean) (ElapsedSeconds :type Float%20%28double-precision%29) (TriggeredSeconds :type Float%20%28double-precision%29) (InputAction :type Input%20Action%20Object%20Reference :default "/Game/00/Inputs/IA_Jump.IA_Jump"))
  (:Started
    (Character|Jump))
  (:Completed
    (Character|StopJumping)))

(event EventBeginPlay
  (Utilities|FlowControl|Sequence
    (:then_0
      (if (Pawn|IsLocallyControlled)
        (if (Utilities|IsValid (PlayerController|LocalPlayerSubsystems|GetEnhancedInputLocalPlayerSubsystem (Game|GetPlayerController 0)))
          (Utilities|Time|SetTimerbyFunctionName 0 "SetPlayerHeight" 5.0)
          (Input|AddMappingContext (PlayerController|LocalPlayerSubsystems|GetEnhancedInputLocalPlayerSubsystem (Game|GetPlayerController 0)) "/Game/00/Inputs/IMC_BasePawnMovement.IMC_BasePawnMovement" 0 "(bIgnoreAllPressedKeysUntilRelease=True,bForceImmediately=False,bNotifyUserSettings=False)"))))
    (:then_1
      (CallFunction|TrackerReplication))))

(event EventTick
  (params (DeltaSeconds :type Float%20%28single-precision%29))
  (CallFunction|OffsetActortoHMD)
  (CallFunction|ScaleActortoHMD)
  (CallFunction|InterpolateTrackingSources))

(fn ConstructionScript)

(fn OffsetActortoHMD
  (bind _playerheight (Variables|Default|GetPlayerHeight))
  (bind _camera (Variables|Default|GetCamera))
  (bind _capsulecomponent (Variables|Collision|GetCapsuleComponent))
  (bind _returnvalue (Transformation|GetWorldLocation _capsulecomponent))
  (bind _returnvalue_2 (Transformation|GetWorldLocation _camera))
  (bind _returnvalue_3 (/ _playerheight 2.0))
  (bind _returnvalue_4 (- (.z _returnvalue_2) (.z _returnvalue)))
  (bind _returnvalue_5 (- (Math|Vector|MakeVector (.x _returnvalue_2) (.y _returnvalue_2) 0.0) (Math|Vector|MakeVector (.x _returnvalue) (.y _returnvalue) 0.0)))
  (Variables|Default|SetCurrentHeightOffset (- _returnvalue_4 _returnvalue_3))
  (if (not (> _returnvalue_4 (+ _returnvalue_3 5.0)))
    (Transformation|AddWorldOffset (Variables|Collision|GetCapsuleComponent) _returnvalue_5 true false)
    (Transformation|AddWorldOffset (Variables|Default|GetVROrigin) (Math|Vector|NegateVector _returnvalue_5) false false)))

(fn ScaleActortoHMD
  (bind _capsulecomponent (Variables|Collision|GetCapsuleComponent))
  (bind _camera (Variables|Default|GetCamera))
  (bind _vrorigin (Variables|Default|GetVROrigin))
  (bind _relativelocation (Variables|/Script/Engine.SceneComponent|GetRelativeLocation _camera))
  (bind _relativelocation_2 (Variables|/Script/Engine.SceneComponent|GetRelativeLocation _vrorigin))
  (bind _returnvalue (/ (.z _relativelocation) 2.0))
  (if (< (.z _relativelocation) (Variables|Default|GetPlayerHeight))
    (Components|Capsule|SetCapsuleSize _capsulecomponent (Class|CapsuleComponent|GetUnscaledCapsuleRadius _capsulecomponent) _returnvalue true)
    (Transformation|SetRelativeLocation _vrorigin (Math|Vector|MakeVector (.x _relativelocation_2) (.y _relativelocation_2) (- (* _returnvalue -1.0) 2.15)) false false)))

(fn SetPlayerHeight
  (Variables|Default|SetPlayerHeight (.z (Variables|/Script/Engine.SceneComponent|GetRelativeLocation (Variables|Default|GetCamera)))))