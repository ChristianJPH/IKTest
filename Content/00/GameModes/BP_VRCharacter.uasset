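; BP_VRCharacter is, despite its name, a game mode Blueprint that hands pawn role assignment to a role manager.
; BeginPlay constructs a BP_RoleManager object.
; PostLogin binds each new player's possessed-pawn-changed event, stores the controller and prints the player count.
; When that event fires, the new pawn is passed to the role manager's SetRole.
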(event Custom|OnPosses
  (params (OldPawn :type Pawn%20Object%20Reference) (NewPawn :type Pawn%20Object%20Reference))
  (Default|SetRole (Variables|Default|GetRoleManager) NewPawn))

(event EventBeginPlay
  (bind _returnvalue (Game|ConstructObjectfromClass "/Game/00/Blueprints/BP_RoleManager.BP_RoleManager_C"))
  (Variables|Default|SetRoleManager _returnvalue))

(event EventTick
  (params (DeltaSeconds :type Float%20%28single-precision%29)))

(event EventPostLogin
  (params (NewPlayer :type Player%20Controller%20Object%20Reference))
  (bind _playercontrollers (Variables|Default|GetPlayerControllers))
  (Pawn|BindEventtoOnPossessedPawnChanged NewPlayer (delegate Custom|OnPosses))
  (Utilities|Array|Add _playercontrollers NewPlayer)
  (Development|PrintString (Utilities|String|ToString(Integer) (Utilities|Array|Length _playercontrollers)) true true "(R=1.000000,G=0.000201,B=0.886573,A=1.000000)" 5.0))

(fn ConstructionScript)